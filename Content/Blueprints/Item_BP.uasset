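; Item_BP is an interactable item that the player uses with the E key while standing in its Box trigger.
; When BP_ThirdPersonCharacter enters and ShowItem is true, it creates an E_UI prompt widget and enables input on itself.
; Pressing E swaps the mesh to SM_Emtryitem and clears ShowItem, making the interaction one-shot.
; Leaving the box removes the widget and disables input.
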(event OnComponentBeginOverlap(Box)
  (params (OverlappedComponent :type Primitive%20Component%20Object%20Reference) (OtherActor :type Actor%20Object%20Reference) (OtherComp :type Primitive%20Component%20Object%20Reference) (OtherBodyIndex :type Integer) (bFromSweep :type Boolean) (SweepResult :type Hit%20Result%20Structure%20%28by%20ref%29))
  (bind _returnvalue (Game|GetPlayerController 0))
  (Utilities|Casting|CastToBP_ThirdPersonCharacter OtherActor)
  (if (Variables|Default|GetShowItem?)
    (bind _returnvalue_2 (UserInterface|CreateWidget "/Game/Widgets/E_UI.E_UI_C" _returnvalue))
    (bind _output_get (Variables|Default|SetShowUI _returnvalue_2))
    (UserInterface|Viewport|AddtoViewport _output_get 0)
    (Input|EnableInput _returnvalue)))

(event OnComponentEndOverlap(Box)
  (params (OverlappedComponent :type Primitive%20Component%20Object%20Reference) (OtherActor :type Actor%20Object%20Reference) (OtherComp :type Primitive%20Component%20Object%20Reference) (OtherBodyIndex :type Integer))
  (Utilities|Casting|CastToBP_ThirdPersonCharacter OtherActor)
  (Widget|RemovefromParent (Variables|Default|GetShowUI))
  (Input|DisableInput (Game|GetPlayerController 0)))

(event Input|KeyboardEvents|E
  (params (Key :type Key%20Structure :default "None"))
  (:Pressed
    ;[1 1 1] Branch or Doonce
    (if (Variables|Default|GetShowItem?)
      (Components|StaticMesh|SetStaticMesh (Variables|Debug|GetStaticMeshComponent) "/Game/Fantastic_Village_Pack/meshes/props/container/SM_Emtryitem.SM_Emtryitem")
      (Variables|Default|SetShowItem? false))))

(fn ConstructionScript)