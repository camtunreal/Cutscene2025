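; Food_BP2 is a collectable food source that shows an interaction prompt when the third-person character comes near.
; Entering its Box trigger creates an F_UI widget and adds it to the viewport, and leaving removes it.
; The CollectItem event, with no caller in this graph, swaps the mesh to an empty-food model and clears Hasfood, so it takes effect only while food remains.
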(event OnComponentBeginOverlap(Box)
  (params (OverlappedComponent :type Primitive%20Component%20Object%20Reference) (OtherActor :type Actor%20Object%20Reference) (OtherComp :type Primitive%20Component%20Object%20Reference) (OtherBodyIndex :type Integer) (bFromSweep :type Boolean) (SweepResult :type Hit%20Result%20Structure%20%28by%20ref%29))
  (Utilities|Casting|CastToBP_ThirdPersonCharacter OtherActor)
  (bind _returnvalue (UserInterface|CreateWidget "/Game/Widgets/F_UI.F_UI_C" (Game|GetPlayerController 0)))
  (bind _output_get (Variables|Default|SetShow%20UI _returnvalue))
  (UserInterface|Viewport|AddtoViewport _output_get 0))

(event OnComponentEndOverlap(Box)
  (params (OverlappedComponent :type Primitive%20Component%20Object%20Reference) (OtherActor :type Actor%20Object%20Reference) (OtherComp :type Primitive%20Component%20Object%20Reference) (OtherBodyIndex :type Integer))
  (Utilities|Casting|CastToBP_ThirdPersonCharacter OtherActor)
  (Widget|RemovefromParent (Variables|Default|GetShow%20UI)))

(event Custom|CollectItem
  (if (Variables|Default|GetHasfood?)
    (Components|StaticMesh|SetStaticMesh (Variables|Debug|GetStaticMeshComponent) "/Game/Fantastic_Village_Pack/meshes/props/food/SM_Emtry_Food.SM_Emtry_Food")
    (Variables|Default|SetHasfood? false)))

(fn ConstructionScript)