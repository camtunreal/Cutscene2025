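; FoodItem_BP is an interactable food prop that the player can empty by pressing E while nearby.
; A Box overlap with BP_ThirdPersonCharacter shows an EKey_UI prompt and enables input on the actor; leaving removes the prompt and disables input.
; Pressing E prints a debug "Hello" and swaps the static mesh to EmptyFood_SM.
; Nothing marks the item as used, so the prompt still appears afterwards.
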(event OnComponentBeginOverlap(Box)
  (params (OverlappedComponent :type Primitive%20Component%20Object%20Reference) (OtherActor :type Actor%20Object%20Reference) (OtherComp :type Primitive%20Component%20Object%20Reference) (OtherBodyIndex :type Integer) (bFromSweep :type Boolean) (SweepResult :type Hit%20Result%20Structure%20%28by%20ref%29))
  (bind _returnvalue (Game|GetPlayerController 0))
  (Utilities|Casting|CastToBP_ThirdPersonCharacter OtherActor)
  (bind _returnvalue_2 (UserInterface|CreateWidget "/Game/Widgets/EKey_UI.EKey_UI_C" _returnvalue))
  (bind _output_get (Variables|Default|SetShowUI _returnvalue_2))
  (UserInterface|Viewport|AddtoViewport _output_get 0)
  (Input|EnableInput _returnvalue))

(event OnComponentEndOverlap(Box)
  (params (OverlappedComponent :type Primitive%20Component%20Object%20Reference) (OtherActor :type Actor%20Object%20Reference) (OtherComp :type Primitive%20Component%20Object%20Reference) (OtherBodyIndex :type Integer))
  (Utilities|Casting|CastToBP_ThirdPersonCharacter OtherActor)
  (Widget|RemovefromParent (Variables|Default|GetShowUI))
  (Input|DisableInput (Game|GetPlayerController 0)))

(event EventBeginPlay)

(event Collision|EventActorBeginOverlap
  (params (OtherActor :type Actor%20Object%20Reference)))

(event EventTick
  (params (DeltaSeconds :type Float%20%28single-precision%29)))

(event Input|KeyboardEvents|E
  (params (Key :type Key%20Structure :default "None"))
  (:Pressed
    (Development|PrintString "Hello")
    (Components|StaticMesh|SetStaticMesh (Variables|Debug|GetStaticMeshComponent) "/Game/Fantastic_Village_Pack/meshes/props/food/EmptyFood_SM.EmptyFood_SM")))

(fn ConstructionScript)